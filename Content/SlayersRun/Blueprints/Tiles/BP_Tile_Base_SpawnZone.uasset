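; Tile Blueprint for SlayersRun that populates a spawn zone with either a coin or an enemy.
; After the parent construction script runs, SpawnObject makes a random two-way pick and adds the matching child actor component.
; The component is placed at a random point inside the SpawnArea box, using its relative location and extent.
; All spawning happens in the construction script, and the event graph is unused.
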(event EventBeginPlay)

(event EventActorBeginOverlap
  (params (OtherActor :type Actor%20Object%20Reference)))

(event EventTick
  (params (DeltaSeconds :type Float%20%28single-precision%29)))

(fn ConstructionScript
  (|CallParentFunction)
  (CallFunction|SpawnObject))

(fn SpawnObject
  (bind _spawn_area (Variables|Default|GetSpawn%20Area))
  (bind _relativelocation (Variables|/Script/Engine.SceneComponent|GetRelativeLocation _spawn_area))
  (bind _boxextent (Variables|/Script/Engine.BoxComponent|GetBoxExtent _spawn_area))
  (bind _returnvalue (Math|Random|RandomPointinBoundingBox _relativelocation _boxextent))
  (bind _returnvalue_2 (Math|Conversions|ToTransform(Vector) _returnvalue))
  (switch int (Math|Random|RandomIntegerinRange 0 1) ; Switch Coin / enemy
    (:0
      (AddComponent|AddChildActorComponent false _returnvalue_2))
    (:1
      (AddComponent|AddChildActorComponent false _returnvalue_2))))