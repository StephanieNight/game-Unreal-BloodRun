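; Base floor tile for an endless runner, exposing its AttachPoint transform, likely for chaining the next tile.
; When the RunCharacter leaves EndTrigger, the tile asks RunnerGameMode to add a floor tile, then destroys itself after a short delay.
; Left and right death walls kill the character only when the hit normal nearly matches its forward vector, using a dot-product test to filter glancing contacts.
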(event OnComponentEndOverlap(EndTrigger)
  (params (OtherActor :type Actor%20Object%20Reference) (OtherComp :type Primitive%20Component%20Object%20Reference) (OtherBodyIndex :type Integer))
  (Utilities|Casting|CastToRunCharacter OtherActor)
  (bind _asrunner_game_mode (Utilities|Casting|CastToRunnerGameMode (Game|GetGameMode)))
  (Default|AddFloorTile _asrunner_game_mode)
  (Utilities|FlowControl|Delay 0.5)
  (Actor|DestroyActor))

(event OnComponentHit(Deathwall_R)
  (params (OtherActor :type Actor%20Object%20Reference) (OtherComp :type Primitive%20Component%20Object%20Reference) (NormalImpulse :type Vector :default "0, 0, 0") (Hit :type Hit%20Result%20Structure%20%28by%20ref%29))
  (bind _asrun_character (Utilities|Casting|CastToRunCharacter OtherActor))
  (if (Math|Float|NearlyEqual(Float) (Math|Vector|DotProduct (.normal Hit) (Transformation|GetActorForwardVector _asrun_character)) 1.0 0.01)
    (Default|Death _asrun_character)))

(event OnComponentHit(Deathwall_L)
  (params (OtherActor :type Actor%20Object%20Reference) (OtherComp :type Primitive%20Component%20Object%20Reference) (NormalImpulse :type Vector :default "0, 0, 0") (Hit :type Hit%20Result%20Structure%20%28by%20ref%29))
  (bind _asrun_character (Utilities|Casting|CastToRunCharacter OtherActor))
  (if (Math|Float|NearlyEqual(Float) (Math|Vector|DotProduct (.normal Hit) (Transformation|GetActorForwardVector _asrun_character)) 1.0 0.01)
    (Default|Death _asrun_character)))

(event EventActorBeginOverlap
  (params (OtherActor :type Actor%20Object%20Reference)))

(event EventTick
  (params (DeltaSeconds :type Float%20%28single-precision%29)))

(event EventBeginPlay)

(fn ConstructionScript)

(fn GetAttachTransform
  (return (Transformation|GetWorldTransform (Variables|Default|GetAttachPoint))))