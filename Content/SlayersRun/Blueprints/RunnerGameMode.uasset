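; Game mode for an endless runner that builds the track from tiles and shows the RunHud widget on BeginPlay.
; It first lays a spawn zone of straight road tiles, chaining each onto the previous tile's attach transform through NextSpawnPoint.
; AddFloorTile, not called within this graph, appends random straight tiles until the count exceeds MaxStraigths.
; It then calls AddFloorCurve, which places a random curve, resets the count and rerolls that limit.
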(event EventBeginPlay
  (bind _returnvalue (UserInterface|CreateWidget "/Game/SlayersRun/UMG/RunHud.RunHud_C"))
  (UserInterface|Viewport|AddtoViewport _returnvalue 0)
  (CallFunction|MakeSpawnZone))

(fn ConstructionScript)

(fn AddFloorTile
  (bind _floortiles (Variables|Default|GetFloorTiles))
  (if (> (Variables|Default|GetCurrentStraigths) (Variables|Default|GetMaxStraigths))
    (CallFunction|AddFloorCurve)
    (else
      (bind _returnvalue (Game|SpawnActorfromClass (Utilities|Array|Get(acopy) _floortiles (Math|Random|RandomIntegerinRange 0 (Utilities|Array|LastIndex _floortiles))) (Variables|Default|GetNextSpawnPoint) "Undefined" 0 0))
      (bind _asbp_tile_base (Utilities|Casting|CastToBP_Tile_Base _returnvalue))
      (bind _attach_transform (Default|GetAttachTransform _asbp_tile_base))
      (Variables|Default|SetNextSpawnPoint _attach_transform)
      (Variables|Default|SetCurrentStraigths (+ (Variables|Default|GetCurrentStraigths) 1)))))

(fn AddFloorCurve
  (bind _floorcurves (Variables|Default|GetFloorCurves))
  (bind _returnvalue (Game|SpawnActorfromClass (Utilities|Array|Get(acopy) _floorcurves (Math|Random|RandomIntegerinRange 0 (Utilities|Array|LastIndex _floorcurves))) (Variables|Default|GetNextSpawnPoint) "Undefined" 0 0))
  (bind _asbp_tile_base (Utilities|Casting|CastToBP_Tile_Base _returnvalue))
  (bind _attach_transform (Default|GetAttachTransform _asbp_tile_base))
  (Variables|Default|SetNextSpawnPoint _attach_transform)
  (Variables|Default|SetCurrentStraigths 0)
  (Variables|Default|SetMaxStraigths (Math|Random|RandomIntegerinRange 7 15)))

(fn MakeSpawnZone
  (for _index (range 0 19)
    (bind _returnvalue (Game|SpawnActorfromClass "/Game/SlayersRun/Blueprints/Tiles/BP_Tile_Road_Straight_01.BP_Tile_Road_Straight_01_C" (Variables|Default|GetNextSpawnPoint) "Undefined" 0 0))
    (bind _attach_transform (Default|GetAttachTransform _returnvalue))
    (Variables|Default|SetNextSpawnPoint _attach_transform)))